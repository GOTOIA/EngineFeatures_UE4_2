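; AI controller for guard NPCs that patrol and attack perceived targets using a behavior tree.
; On begin play it sets up the PatrolData blackboard and runs GuardBehaviour.
; Perception stores any sensed actor without the Enemy tag under EnemyKey and clears it when lost.
; Each tick, a valid focus actor makes the controlled TPCharactere both aim and shoot.
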(event `self.ReceiveBeginPlay`
  ;[1 1 1] Set and use BlackBoard values and Behaviour Tree
  (bind _blackboardcomponent (`self.UseBlackboard` "/Game/Dynamic/NPC/AI/PatrolData.PatrolData"))
  (`self.RunBehaviorTree` "/Game/Dynamic/NPC/AI/GuardBehaviour.GuardBehaviour")
  (set `self.BlackBoardComp` _blackboardcomponent))

(event `self.ReceiveTick`
  (params (DeltaSeconds :type "Float (single-precision)"))
  ;[1 1 1] Set aiming if focus actor is valid
  (bind _astpcharactere (cast `/Game/Dynamic/NPC/Behaviour/TPCharactere` (`self.K2_GetPawn`)))
  (bind _output_get (set `/Game/Dynamic/NPC/Behaviour/TPCharactere.Aiming` (`KismetSystemLibrary.IsValid` (`self.GetFocusActor`)) _astpcharactere))
  (set `/Game/Dynamic/NPC/Behaviour/TPCharactere.Shooting` _output_get _astpcharactere))

(event `self.AIPerception.OnTargetPerceptionUpdated`
  (params (Actor :type "Actor Object Reference") (Stimulus :type "AIStimulus Structure"))
  (bind _blackboardcomp (`self.BlackBoardComp`))
  (bind _enemykey (`self.EnemyKey`))
  ;[1 1 1] Set Perception and values of blackboard key (True or false) when stimulus right
  (if (`self.ActorHasTag` Actor "Enemy")
    _
    (elif (`.bSuccessfullySensed` (break `AIStimulus` Stimulus))
      (`BlackboardComponent.SetValueAsObject` _blackboardcomp _enemykey Actor)
      (else
        (`BlackboardComponent.ClearValue` _blackboardcomp _enemykey)))))

(fn `UserConstructionScript`)